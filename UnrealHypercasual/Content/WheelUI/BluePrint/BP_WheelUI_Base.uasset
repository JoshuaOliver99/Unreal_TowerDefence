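; Base Blueprint for a radial wheel menu that E builds from the player's current Interactor target, one segment per available interaction.
; Spawns W_WheelUI at viewport centre or mouse position, switching input and cursor or look handling by input mode.
; Mouse or stick angle selects segments on Tick outside InputMode1, while arrow/D-pad keys step by on-screen direction.
; Confirming messages the segment and, if unlocked, the interactable's owning actor.
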(event `self.ReceiveTick`
  (params (DeltaSeconds :type "Float (single-precision)"))
  (bind _returnvalue (`KismetMathLibrary.MakeVector2D` (`self.GetInputAxisKeyValue`) (`self.GetInputAxisKeyValue`)))
  (bind (_locationx _locationy) (`WidgetLayoutLibrary.GetMousePositionScaledByDPI` (`self.PlayerController`)))
  (bind (_locationx_2 _locationy_2) (`WidgetLayoutLibrary.GetMousePositionScaledByDPI` (`self.PlayerController`)))
  (bind _returnvalue_2 (`KismetMathLibrary.Distance2D` (`KismetMathLibrary.MakeVector2D` _locationx_2 _locationy_2) (`self.MouseLoc_Start`)))
  (bind _output (`|GetArrayItem` (`/Game/WheelUI/Widget/W_WheelPlate.UI_PieceArr` (`/Game/WheelUI/Widget/W_WheelUI.UI_Plate` (`self.UI_Screen`)))))
  (bind _returnvalue_3 (select `/Game/WheelUI/BluePrint/Enum_InputMode` (`self.InputMode`) :`NewEnumerator0` (`KismetMathLibrary.Normal2D` (- (`KismetMathLibrary.MakeVector2D` _locationx _locationy) (`self.MouseLoc_Start`))) :`NewEnumerator1` _returnvalue))
  (bind _x (`KismetMathLibrary.BreakVector2D` (`.ImageSize` (break `SlateBrush` (`Image.Brush` (`/Game/WheelUI/Widget/W_WheelSegment.Image_Wheel` _output))))))
  (bind _returnvalue_4 (`KismetMathLibrary.DegAcos` (`KismetMathLibrary.DotProduct2D` _returnvalue_3 (1.0 0.0))))
  (if (not (`|EnumEquality` (`self.InputMode`) "NewEnumerator3"))
    (`/Engine/EditorBlueprintResources/StandardMacros.IsValid` (`self.UI_Screen`)
      (:`Is Valid`
        (set `self.CurrentSelectedSegmentIndex` (`KismetMathLibrary.SelectInt` (`.ReturnValue` (`KismetMathLibrary.FMod` (`KismetMathLibrary.FMod` (+ (+ (select `bool` (> (`.Y` (`KismetMathLibrary.BreakVector2D` _returnvalue_3)) 0.0) :`false` _returnvalue_4 :`true` (+ (* _returnvalue_4 -1.0) 360.0)) (/ (/ 360.0 (`KismetMathLibrary.Conv_IntToDouble` (`self.Num Element`))) 2.0)) (`self.Rotate Angle`)) 360.0) (/ 360.0 (`KismetMathLibrary.Conv_IntToDouble` (`self.Num Element`))))) -1 (select `/Game/WheelUI/BluePrint/Enum_InputMode` (`self.InputMode`) :`NewEnumerator0` (and (>= _returnvalue_2 (* (* _x (`/Game/WheelUI/Widget/W_WheelSegment.Radius_In` _output)) (`self.Scale`))) (<= _returnvalue_2 (* (* _x (`/Game/WheelUI/Widget/W_WheelSegment.Radius_Out` _output)) (`self.Scale`)))) :`NewEnumerator1` (>= (`KismetMathLibrary.VSize2D` _returnvalue) 0.4))))))))

(event `self.ReceiveBeginPlay`
  (bind _output_get (set `self.PlayerController` (`GameplayStatics.GetPlayerController` 0)))
  (`self.EnableInput` _output_get))

(event `Key|RightMouseButton`
  (params (Key :type "Key Structure"))
  ;[1 1 1] Input
  (:`Pressed`
    (`/Engine/EditorBlueprintResources/StandardMacros.IsValid` (`self.UI_Screen`)
      (:`Is Valid`
        (`self.UI Destroy Operation` :!label _label)))))

(event `Key|Gamepad_FaceButton_Right`
  (params (Key :type "Key Structure"))
  ;[1 1 1] Input
  (:`Pressed`
    (`/Engine/EditorBlueprintResources/StandardMacros.IsValid` (`self.UI_Screen`) :!label _label_2
      (:`Is Valid`
        (goto _label))
      (:`Is Not Valid`
        (`self.UI Spawn Operation`)))))

(event `Key|E`
  (params (Key :type "Key Structure"))
  (:`Pressed`
    (bind _interactable (`self.Check and setup Interactable`))
    (if _interactable
      (goto _label_2))))

(event `Key|Gamepad_RightTrigger`
  (params (Key :type "Key Structure"))
  ;[1 1 1] Input
  (:`Pressed`
    (goto _label_2))
  (:`Released`
    (`/Engine/EditorBlueprintResources/StandardMacros.IsValid` (`self.UI_Screen`) :!label _label_3
      (:`Is Valid`
        (`self.UI Interact Operation`)))))

(event `Key|LeftMouseButton`
  (params (Key :type "Key Structure"))
  ;[1 1 1] Input
  (:`Pressed`
    (goto _label_3)))

(event `Key|Gamepad_FaceButton_Bottom`
  (params (Key :type "Key Structure"))
  ;[1 1 1] Input
  (:`Pressed`
    (goto _label_3)))

(event `Key|Enter`
  (params (Key :type "Key Structure"))
  ;[1 1 1] Input
  (:`Pressed`
    (goto _label_3)))

(event `Key|Gamepad_DPad_Up`
  (params (Key :type "Key Structure"))
  (bind _currentselectedsegmentindex (`self.CurrentSelectedSegmentIndex`))
  ;[1 1 1] Input
  (:`Pressed`
    (if (`KismetMathLibrary.InRange_FloatFloat` (`KismetMathLibrary.FMod` (+ (* (`self.CurrentSelectedSegmentIndex`) (/ 360.0 (`KismetMathLibrary.Conv_IntToDouble` (`self.Num Element`)))) (`self.Rotate Angle`)) 360.0) 90.0 270.0 false false) :!label _label_4
      (bind _result (`/Engine/EditorBlueprintResources/StandardMacros.DecrementInt` _currentselectedsegmentindex :!label _label_5)
        (:`  `
          (if (< _result 0)
            (set `self.CurrentSelectedSegmentIndex` (+ _result (`self.Num Element`))))))
      (else
        (bind _result_2 (`/Engine/EditorBlueprintResources/StandardMacros.IncrementInt` _currentselectedsegmentindex :!label _label_6)
          (:`  `
            (set `self.CurrentSelectedSegmentIndex` (mod _result_2 (`self.Num Element`)))))))))

(event `Key|Up`
  (params (Key :type "Key Structure"))
  ;[1 1 1] Input
  (:`Pressed`
    (goto _label_4)))

(event `Key|Gamepad_DPad_Down`
  (params (Key :type "Key Structure"))
  ;[1 1 1] Input
  (:`Pressed`
    (if (`KismetMathLibrary.InRange_FloatFloat` (`KismetMathLibrary.FMod` (+ (* (`self.CurrentSelectedSegmentIndex`) (/ 360.0 (`KismetMathLibrary.Conv_IntToDouble` (`self.Num Element`)))) (`self.Rotate Angle`)) 360.0) 90.0 270.0 false false) :!label _label_7
      (goto _label_6)
      (else
        (goto _label_5)))))

(event `Key|Down`
  (params (Key :type "Key Structure"))
  ;[1 1 1] Input
  (:`Pressed`
    (goto _label_7)))

(event `Key|Gamepad_DPad_Left`
  (params (Key :type "Key Structure"))
  ;[1 1 1] Input
  (:`Pressed`
    (if (`KismetMathLibrary.InRange_FloatFloat` (`KismetMathLibrary.FMod` (+ (* (`self.CurrentSelectedSegmentIndex`) (/ 360.0 (`KismetMathLibrary.Conv_IntToDouble` (`self.Num Element`)))) (`self.Rotate Angle`)) 360.0) 0.0 180.0 false false) :!label _label_8
      (goto _label_6)
      (else
        (goto _label_5)))))

(event `Key|Left`
  (params (Key :type "Key Structure"))
  ;[1 1 1] Input
  (:`Pressed`
    (goto _label_8)))

(event `Key|Gamepad_DPad_Right`
  (params (Key :type "Key Structure"))
  ;[1 1 1] Input
  (:`Pressed`
    (if (`KismetMathLibrary.InRange_FloatFloat` (`KismetMathLibrary.FMod` (+ (* (`self.CurrentSelectedSegmentIndex`) (/ 360.0 (`KismetMathLibrary.Conv_IntToDouble` (`self.Num Element`)))) (`self.Rotate Angle`)) 360.0) 0.0 180.0 false false) :!label _label_9
      (goto _label_5)
      (else
        (goto _label_6)))))

(event `Key|Right`
  (params (Key :type "Key Structure"))
  ;[1 1 1] Input
  (:`Pressed`
    (goto _label_9)))

(fn `Check and setup Interactable`
  (returns (Interactable :type Boolean))
  (bind _returnvalue (`Interactor.GetCurrentInteractable` (`self.GetComponentByClass` (`GameplayStatics.GetPlayerPawn` 0) "/Script/UnrealHypercasual.Interactor")))
  (bind _returnvalue_2 (`Interactable.GetAvailableInteractions` _returnvalue))
  ;[1 1 1] Return false if we're not currently looking at an Interactable
  (`/Engine/EditorBlueprintResources/StandardMacros.IsValid` _returnvalue
    (:`Is Valid`
      ;[1 1 1] Set number of segments
      (set `self.Num Element` (`KismetArrayLibrary.Array_Length` _returnvalue_2))
      ;[1 1 1] Clear any existing UI element data
      (`KismetArrayLibrary.Array_Clear` (`self.Element Arr`))
      ;[1 1 1] Clear any Button Actions
      (`KismetArrayLibrary.Array_Clear` (`self.InteractActor`))
      (for _array_element _returnvalue_2
        (`KismetSystemLibrary.PrintString` "Item")
        ;[1 1 1] Create and store UI element data
        (`KismetArrayLibrary.Array_Add` (`self.Element Arr`) (make `/Game/WheelUI/BluePrint/S_Element` (`Interaction.GetThumbnail` _array_element) (`KismetTextLibrary.Conv_StringToText` (`Interaction.GetTitle` _array_element))))
        ;[1 1 1] Store Actors For Button Events
        (`KismetArrayLibrary.Array_Add` (`self.InteractActor`) (`ActorComponent.GetOwner` (`Interactor.GetCurrentInteractable` (`self.GetComponentByClass` (`GameplayStatics.GetPlayerPawn` 0) "/Script/UnrealHypercasual.Interactor")))))
      (return true))
    (:`Is Not Valid`
      (return false))))

(fn `UI Destroy Operation`
  ;[1 1 1] remove UI from viewport
  (`Widget.RemoveFromParent` (`self.UI_Screen`))
  ;[1 1 1] set varible to empty
  (set `self.UI_Screen` null)
  (`WidgetBlueprintLibrary.SetInputMode_GameOnly` (`self.PlayerController`))
  (switch `/Game/WheelUI/BluePrint/Enum_InputMode` (`self.InputMode`)
    (:`NewEnumerator0`
      ;[1 0 0] set mouse cursor
      (set `PlayerController.bShowMouseCursor` false (`self.PlayerController`)))
    (:`NewEnumerator1`
      (`Controller.SetIgnoreLookInput` (`self.PlayerController`) false))))

(fn `UI Interact Operation`
  (bind _currentselectedsegmentindex (`self.CurrentSelectedSegmentIndex`))
  (bind _output (`|GetArrayItem` (`/Game/WheelUI/Widget/W_WheelPlate.UI_PieceArr` (`/Game/WheelUI/Widget/W_WheelUI.UI_Plate` (`self.UI_Screen`))) (`self.CurrentSelectedSegmentIndex`)))
  ;[1 1 1] Judge if a segment is selected. If not, destroy UI
  (if (>= (`self.CurrentSelectedSegmentIndex`) 0)
    (`|ExecutionSequence`
      (:`then_0`
        ;[1 1 1] Judge if the selected segment is locked
        (if (`/Game/WheelUI/Widget/W_WheelSegment.Is locked` _output)
          ;[1 1 1] Call implement events of selected UI segment
          (message `/Game/WheelUI/BluePrint/BPI_UI.Interaction_Locked` _output (`self.CurrentSelectedSegmentIndex`))
          (return)
          (else
            (message `/Game/WheelUI/BluePrint/BPI_UI.Interaction` _output _currentselectedsegmentindex)
            (if (>= _currentselectedsegmentindex (`KismetArrayLibrary.Array_Length` (`self.InteractActor`)))
              (`KismetSystemLibrary.PrintString` "Unknown Interactive Object" true true (struct :`R` 1.0 :`G` 0.369887 :`B` 0.158568 :`A` 1.0))
              (else
                ;[1 1 1] call implement event of other actors
                (message `/Game/WheelUI/BluePrint/BPI_UI.Interaction` (`|GetArrayItem` (`self.InteractActor`) _currentselectedsegmentindex) (`self.CurrentSelectedSegmentIndex`)))))))
      (:`then_1`
        (`self.UI Destroy Operation` :!label _label)))
    (else
      (goto _label))))

(fn `UI Spawn Operation`
  (bind (_locationx _locationy) (`WidgetLayoutLibrary.GetMousePositionScaledByDPI` (`self.PlayerController`)))
  (if (`self.ConfirmSpawnLocation`)
    (set `self.MouseLoc_Start` (+ (/ (/ (`WidgetLayoutLibrary.GetViewportSize`) 2.0) (`WidgetLayoutLibrary.GetViewportScale`)) (`self.Offset_UI`)))
    (else
      (set `self.MouseLoc_Start` (`KismetMathLibrary.MakeVector2D` _locationx _locationy))))
  ;[1 1 1] Spawn UI
  (bind _returnvalue (`|CreateWidget` "/Game/WheelUI/Widget/W_WheelUI.W_WheelUI_C" (`self.PlayerController`) (`self.MouseLoc_Start`) (`self.Element Arr`) (`self.Num Element`) (`self.Rotate Angle`) (`self.Scale`) (`self.Text Offset Title`) (`self.Text Offset Description`) (`self.Material Wheel Default`) (`self.Material Wheel Selected`) (`self.Material Text Default`) (`self.Material Text Selected`) (`self.Material Icon`) (`self.Element Cancel`)))
  (bind _output_get (set `self.UI_Screen` _returnvalue))
  (`UserWidget.AddToViewport` _output_get 0)
  (`WidgetBlueprintLibrary.SetInputMode_GameAndUIEx` (`self.PlayerController`) null)
  (switch `/Game/WheelUI/BluePrint/Enum_InputMode` (`self.InputMode`)
    (:`NewEnumerator0`
      ;[1 0 0] set mouse cursor
      (set `PlayerController.bShowMouseCursor` true (`self.PlayerController`)))
    (:`NewEnumerator1`
      (`Controller.SetIgnoreLookInput` (`self.PlayerController`) true))))

(fn `UserConstructionScript`)